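; BP_FleshPiece is a short-lived gore chunk actor.
; On BeginPlay it launches its Model mesh upward with a physics force and randomly picks one of three flesh meshes.
; After a ten-second delay, the SizeDown timeline drives the mesh's world scale, and the actor destroys itself when the timeline finishes.
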(event `self.ReceiveBeginPlay`
  (`PrimitiveComponent.AddForce` (`self.Model`) (0.0 0.0 100000.0) "None" false)
  (switch `int` (`KismetMathLibrary.RandomInteger` 3)
    (:`0`
      (`StaticMeshComponent.SetStaticMesh` (`self.Model`) "/Game/Meshes/Enemies/SM_Flesh1.SM_Flesh1"))
    (:`1`
      (`StaticMeshComponent.SetStaticMesh` (`self.Model`) "/Game/Meshes/Enemies/SM_Flesh2.SM_Flesh2"))
    (:`2`
      (`StaticMeshComponent.SetStaticMesh` (`self.Model`) "/Game/Meshes/Enemies/SM_Flesh3.SM_Flesh3")))
  (`KismetSystemLibrary.Delay` 10.0)
  (bind (_direction _scale) (`Timeline|SizeDown`)
    (:`Update`
      (`SceneComponent.SetWorldScale3D` (`self.Model`) _scale))
    (:`Finished`
      (`self.K2_DestroyActor`))))

(fn `UserConstructionScript`)