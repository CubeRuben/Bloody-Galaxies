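; BP_Door is a door actor with open, close, lock and unlock events, each playing a sound at the door's location.
; The DoorAnimation timeline slides the top part and two mirrored bottom parts, reversing to close.
; The LockAnimation timeline moves the lock mesh, reversing to unlock.
; The lock mesh is hidden at BeginPlay, shown on locking and hidden again when the reverse finishes.
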(event `self.OpenDoor`
  (`GameplayStatics.PlaySoundAtLocation` "/Game/Audio/Ship/Door/SC_DoorOpenClose.SC_DoorOpenClose" (`SceneComponent.K2_GetComponentLocation` (`self.RootComponent`)) (struct) 1.0 1.0 0.0 null null null null)
  (bind (_direction _bottomoffset _topoffset) (`Timeline|DoorAnimation` :!label _label)
    (:`Update`
      (`SceneComponent.K2_SetRelativeLocation` (`self.SM_DoorPartBottom1`) _bottomoffset false false)
      (`SceneComponent.K2_SetRelativeLocation` (`self.SM_DoorPartBottom`) (* _bottomoffset (`KismetMathLibrary.Conv_DoubleToVector` -1.0)) false false)
      (`SceneComponent.K2_SetRelativeLocation` (`self.SM_DoorPartTop`) _topoffset false false))))

(event `self.CloseDoor`
  (`GameplayStatics.PlaySoundAtLocation` "/Game/Audio/Ship/Door/SC_DoorOpenClose.SC_DoorOpenClose" (`SceneComponent.K2_GetComponentLocation` (`self.RootComponent`)) (struct) 1.0 1.0 0.0 null null null null)
  (goto _label :!via `Reverse`))

(event `self.LockDoor`
  (`SceneComponent.SetVisibility` (`self.SM_DoorLock`) true false)
  (`GameplayStatics.PlaySoundAtLocation` "/Game/Audio/Ship/Door/SC_DoorLock.SC_DoorLock" (`SceneComponent.K2_GetComponentLocation` (`self.RootComponent`)) (struct) 1.0 1.0 0.0 null null null null)
  (bind (_direction _lock) (`Timeline|LockAnimation` :!label _label_2)
    (:`Update`
      (`SceneComponent.K2_SetRelativeLocation` (`self.SM_DoorLock`) _lock false false))
    (:`Finished`
      (switch `ETimelineDirection` _direction
        (:`Backward`
          (`SceneComponent.SetVisibility` (`self.SM_DoorLock`) false false :!label _label_3))))))

(event `self.UnlockDoor`
  (`GameplayStatics.PlaySoundAtLocation` "/Game/Audio/Ship/Door/SC_DoorLock.SC_DoorLock" (`SceneComponent.K2_GetComponentLocation` (`self.RootComponent`)) (struct) 1.0 1.0 0.0 null null null null)
  (goto _label_2 :!via `Reverse`))

(event `self.ReceiveBeginPlay`
  (goto _label_3))

(fn `UserConstructionScript`)