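; BP_AcidSplash is a temporary acid hazard that damages the player while they stand in it.
; On spawn it gives its decal a dynamic material with a randomized Z parameter, waits, then drives Opacity from a timeline and destroys itself when that finishes.
; Entering the box applies an initial hit and starts a looping timer for repeated heavier damage, which is cleared on exit.
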(event `self.ReceiveBeginPlay`
  (bind _returnvalue (`KismetMaterialLibrary.CreateDynamicMaterialInstance` "/Game/Materials/M_AcidSplash.M_AcidSplash"))
  (`DecalComponent.SetDecalMaterial` (`self.Decal`) _returnvalue)
  (set `self.Material` _returnvalue)
  (`MaterialInstanceDynamic.SetScalarParameterValue` _returnvalue "Z" (`KismetMathLibrary.RandomFloatInRange` -100.0 100.0))
  (`KismetSystemLibrary.Delay` 10.0)
  (bind (_direction _opacity) (`Timeline|Opacity`)
    (:`Update`
      (`MaterialInstanceDynamic.SetScalarParameterValue` (`self.Material`) "Opacity" _opacity))
    (:`Finished`
      (`self.K2_DestroyActor`))))

(event `self.Box.OnComponentBeginOverlap`
  (params (OverlappedComponent :type "PrimitiveComponent Object Reference") (OtherActor :type "Actor Object Reference") (OtherComp :type "PrimitiveComponent Object Reference") (OtherBodyIndex :type Integer) (bFromSweep :type Boolean) (SweepResult :type "HitResult Structure (by ref)"))
  (bind _asplayer_pawn (cast `PlayerPawn` OtherActor))
  (set `self.Player` _asplayer_pawn)
  (bind _returnvalue (`KismetSystemLibrary.K2_SetTimerDelegate` (delegate `PlayerDamage`) 0.25 true))
  (set `self.DamageTimer` _returnvalue)
  (`PlayerPawn.ApplyDamage` (`self.Player`) 1.0))

(event `self.Box.OnComponentEndOverlap`
  (params (OverlappedComponent :type "PrimitiveComponent Object Reference") (OtherActor :type "Actor Object Reference") (OtherComp :type "PrimitiveComponent Object Reference") (OtherBodyIndex :type Integer))
  (cast `PlayerPawn` OtherActor)
  (set `self.Player` null)
  (`KismetSystemLibrary.K2_ClearAndInvalidateTimerHandle` (`self.DamageTimer`)))

(event `PlayerDamage`
  (`PlayerPawn.ApplyDamage` (`self.Player`) 3.0))

(fn `UserConstructionScript`)