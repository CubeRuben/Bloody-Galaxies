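; BP_Eye is an eyeball actor that blinks periodically and tracks a nearby player pawn.
; Sphere overlaps set and clear the Player reference; Tick rotates the eye mesh using a look-at from player to eye root, or resets its relative rotation when no player is set.
; A looping timer with varied initial delay plays a timeline that pitches two eyelid meshes, the second rolled 180 degrees, to blink.
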(event `Blink`
  (bind (_direction _rotation) (`Timeline|BlinkTimeline` :!via `PlayFromStart`)
    (:`Update`
      (`SceneComponent.K2_SetRelativeRotation` (`self.SM_Eyelid`) (`KismetMathLibrary.MakeRotator` 0.0 (* _rotation -1.0)) false false)
      (`SceneComponent.K2_SetRelativeRotation` (`self.SM_Eyelid1`) (`KismetMathLibrary.MakeRotator` 180.0 _rotation) false false))))

(event `self.ReceiveBeginPlay`
  (`KismetSystemLibrary.K2_SetTimerDelegate` (delegate `Blink`) 5.0 true 1.0 5.0))

(event `self.ReceiveTick`
  (params (DeltaSeconds :type "Float (single-precision)"))
  (`/Engine/EditorBlueprintResources/StandardMacros.IsValid` (`self.Player`)
    (:`Is Valid`
      (`SceneComponent.K2_SetWorldRotation` (`self.SM_Eye`) (`KismetMathLibrary.FindLookAtRotation` (`self.K2_GetActorLocation` (`self.Player`)) (`SceneComponent.K2_GetComponentLocation` (`self.DefaultSceneRoot`))) false false))
    (:`Is Not Valid`
      (`SceneComponent.K2_SetRelativeRotation` :`self` (`self.SM_Eye`)))))

(event `self.Sphere.OnComponentBeginOverlap`
  (params (OverlappedComponent :type "PrimitiveComponent Object Reference") (OtherActor :type "Actor Object Reference") (OtherComp :type "PrimitiveComponent Object Reference") (OtherBodyIndex :type Integer) (bFromSweep :type Boolean) (SweepResult :type "HitResult Structure (by ref)"))
  (bind _asplayer_pawn (cast `PlayerPawn` OtherActor))
  (set `self.Player` _asplayer_pawn))

(event `self.Sphere.OnComponentEndOverlap`
  (params (OverlappedComponent :type "PrimitiveComponent Object Reference") (OtherActor :type "Actor Object Reference") (OtherComp :type "PrimitiveComponent Object Reference") (OtherBodyIndex :type Integer))
  (cast `PlayerPawn` OtherActor)
  (set `self.Player` null))

(fn `UserConstructionScript`)