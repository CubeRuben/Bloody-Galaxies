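; BP_Splinker is an enemy that lobs physics projectiles at the player while they are inside its PlayerDetection volume.
; A looping timer fires ShootToPlayer, launching along GetShootAngle's ballistic arc, solved from distance, gravity and LaunchVelocity without height compensation.
; Tick bends two neck bones toward that launch vector in component space, the bottom at half tilt.
; On destruction it plays a death sound and spawns flesh pieces.
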(event `self.ReceiveTick`
  (params (DeltaSeconds :type "Float (single-precision)"))
  (bind (_returnvalue_roll _returnvalue_pitch _returnvalue_yaw) (`KismetMathLibrary.BreakRotator` (`KismetMathLibrary.MakeRotFromZ` (`KismetMathLibrary.Normal` (`self.GetShootAngle`)))))
  (bind _returnvalue (* (`KismetMathLibrary.DegCos` _returnvalue_yaw) _returnvalue_roll))
  (bind _returnvalue_2 (* _returnvalue_roll (`KismetMathLibrary.DegSin` (* _returnvalue_yaw -1.0))))
  (`/Engine/EditorBlueprintResources/StandardMacros.IsValid` (`self.PlayerPawn`)
    (:`Is Valid`
      (`PoseableMeshComponent.SetBoneRotationByName` (`self.Splinker`) "NeckBottom" (`KismetMathLibrary.MakeRotator` (+ (/ _returnvalue_2 2.0) 90.0) (/ _returnvalue 2.0)) "ComponentSpace")
      (`PoseableMeshComponent.SetBoneRotationByName` (`self.Splinker`) "NeckTop" (`KismetMathLibrary.MakeRotator` (+ _returnvalue_2 90.0) _returnvalue) "ComponentSpace"))))

(event `self.PlayerDetection.OnComponentBeginOverlap`
  (params (OverlappedComponent :type "PrimitiveComponent Object Reference") (OtherActor :type "Actor Object Reference") (OtherComp :type "PrimitiveComponent Object Reference") (OtherBodyIndex :type Integer) (bFromSweep :type Boolean) (SweepResult :type "HitResult Structure (by ref)"))
  (bind _asplayer_pawn (cast `PlayerPawn` OtherActor))
  (set `self.PlayerPawn` _asplayer_pawn)
  (bind _returnvalue (`KismetSystemLibrary.K2_SetTimer` null "ShootToPlayer" 1.0 true 1.0))
  (set `self.ShootingTimer` _returnvalue))

(event `self.PlayerDetection.OnComponentEndOverlap`
  (params (OverlappedComponent :type "PrimitiveComponent Object Reference") (OtherActor :type "Actor Object Reference") (OtherComp :type "PrimitiveComponent Object Reference") (OtherBodyIndex :type Integer))
  (cast `PlayerPawn` OtherActor)
  (`KismetSystemLibrary.K2_ClearAndInvalidateTimerHandle` (`self.ShootingTimer`))
  (set `self.PlayerPawn` null))

(event `self.ReceiveDestroyed`
  (`GameplayStatics.PlaySoundAtLocation` "/Game/Audio/Enemies/Splinker/SC_Death.SC_Death" (`SceneComponent.K2_GetComponentLocation` (`self.RootComponent`)) (struct) 1.0 1.0 0.0 null null null null)
  (for _ (range 8)
    (`|SpawnActorFromClass` "/Game/Blueprints/BP_FleshPiece.BP_FleshPiece_C" (`KismetMathLibrary.MakeTransform` (+ (`self.K2_GetActorLocation`) (0.0 0.0 20.0))) "AlwaysSpawn" "OverrideRootScale" null null)))

(fn `GetShootAngle`
  (returns (ReturnValue :type "Vector Structure"))
  (bind _returnvalue (`self.K2_GetActorLocation` (`self.PlayerPawn`)))
  (bind _returnvalue_2 (`SceneComponent.K2_GetComponentLocation` (`self.LaunchPoint`)))
  (bind (_returnvalue_roll _returnvalue_pitch _returnvalue_yaw) (`KismetMathLibrary.BreakRotator` (`KismetMathLibrary.FindLookAtRotation` _returnvalue_2 _returnvalue)))
  (return (`KismetMathLibrary.RotateAngleAxis` (`KismetMathLibrary.RotateAngleAxis` (`KismetMathLibrary.MakeVector` 0.0 0.0 (`self.LaunchVelocity`)) (/ (`KismetMathLibrary.DegAsin` (* (/ (* (`KismetMathLibrary.VSize` (- _returnvalue _returnvalue_2)) -980.0) (* (`KismetMathLibrary.MultiplyMultiply_FloatFloat` (`self.LaunchVelocity`) 2.0) 2.0)) 2.0)) 2.0) (0.0 -1.0 0.0)) _returnvalue_yaw (0.0 0.0 1.0))))

(fn `ShootToPlayer`
  (`GameplayStatics.PlaySoundAtLocation` "/Game/Audio/Enemies/Splinker/SC_Shot.SC_Shot" (`SceneComponent.K2_GetComponentLocation` (`self.LaunchPoint`)) (struct) 1.0 1.0 1.0 null null null null)
  (bind _returnvalue (`|SpawnActorFromClass` "/Game/Blueprints/Enemies/BP_SplinkerProjectile.BP_SplinkerProjectile_C" (`KismetMathLibrary.MakeTransform` (`SceneComponent.K2_GetComponentLocation` (`self.LaunchPoint`))) "AlwaysSpawn" "OverrideRootScale" null null))
  (`PrimitiveComponent.SetPhysicsLinearVelocity` (`Projectile.MeshComponent` _returnvalue) (`self.GetShootAngle`) false "None"))

(fn `UserConstructionScript`)