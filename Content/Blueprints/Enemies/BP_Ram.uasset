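; BP_Ram is a physics-driven rolling enemy that chases the player within its detection volume and otherwise jitters on random forces.
; Tick accelerates the sphere, toggles roll audio by speed, and hops it upward if it stalls.
; A second trigger plays an attack sound and a timeline that resizes spikes and collider, reversing on exit.
; Player hits deal momentum-based damage, knockback and clamped recoil; destruction spawns flesh pieces with a sound.
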(event `self.ReceiveTick`
  (params (DeltaSeconds :type "Float (single-precision)"))
  (bind _sc_roll (`self.SC_Roll`))
  (bind _sphere (`self.Sphere`))
  (bind _movingforce (`self.MovingForce`))
  (if (> (`KismetMathLibrary.VSizeSquared` (`SceneComponent.GetComponentVelocity` (`self.Sphere`))) 250000.0)
    (if (not (`AudioComponent.IsPlaying` _sc_roll))
      (`AudioComponent.Play` _sc_roll 0.0))
    (else
      (`AudioComponent.Stop` _sc_roll)))
  (`/Engine/EditorBlueprintResources/StandardMacros.IsValid` (`self.Player`)
    (:`Is Valid`
      (`PrimitiveComponent.AddForce` _sphere (* (`KismetMathLibrary.Normal` (* (- (`self.K2_GetActorLocation` (`self.Player`)) (`SceneComponent.K2_GetComponentLocation` (`self.Sphere`))) (1.0 1.0 0.0))) (`KismetMathLibrary.MakeVector` _movingforce _movingforce _movingforce)) "None" true))
    (:`Is Not Valid`
      (`PrimitiveComponent.AddForce` _sphere (* (`self.MovingForce`) (`KismetMathLibrary.RandomUnitVector`)) "None" true)))
  (if (< (`KismetMathLibrary.VSizeSquared` (`SceneComponent.GetComponentVelocity` _sphere)) 10.0)
    (`KismetSystemLibrary.Delay` 1.0)
    (if (< (`KismetMathLibrary.VSizeSquared` (`SceneComponent.GetComponentVelocity` (`self.Sphere`))) 100.0)
      (`PrimitiveComponent.AddImpulse` (`self.Sphere`) (0.0 0.0 1000.0) "None" true))))

(event `self.PlayerDetection.OnComponentBeginOverlap`
  (params (OverlappedComponent :type "PrimitiveComponent Object Reference") (OtherActor :type "Actor Object Reference") (OtherComp :type "PrimitiveComponent Object Reference") (OtherBodyIndex :type Integer) (bFromSweep :type Boolean) (SweepResult :type "HitResult Structure (by ref)"))
  (bind _asplayer_pawn (cast `PlayerPawn` OtherActor))
  (set `self.Player` _asplayer_pawn))

(event `self.PlayerDetection.OnComponentEndOverlap`
  (params (OverlappedComponent :type "PrimitiveComponent Object Reference") (OtherActor :type "Actor Object Reference") (OtherComp :type "PrimitiveComponent Object Reference") (OtherBodyIndex :type Integer))
  (cast `PlayerPawn` OtherActor)
  (set `self.Player` null))

(event `self.PlayerPrepareAtack.OnComponentBeginOverlap`
  (params (OverlappedComponent :type "PrimitiveComponent Object Reference") (OtherActor :type "Actor Object Reference") (OtherComp :type "PrimitiveComponent Object Reference") (OtherBodyIndex :type Integer) (bFromSweep :type Boolean) (SweepResult :type "HitResult Structure (by ref)"))
  (cast `PlayerPawn` OtherActor)
  (`AudioComponent.Play` (`self.SC_Atack`) 0.0)
  (bind (_direction _colliderrange _spikessize) (`Timeline|OpenSpikes` :!label _label)
    (:`Update`
      (`SphereComponent.SetSphereRadius` (`self.Sphere`) _colliderrange true)
      (`SceneComponent.SetWorldScale3D` (`self.SM_RamSpikes`) (`KismetMathLibrary.MakeVector` _spikessize _spikessize _spikessize)))))

(event `self.PlayerPrepareAtack.OnComponentEndOverlap`
  (params (OverlappedComponent :type "PrimitiveComponent Object Reference") (OtherActor :type "Actor Object Reference") (OtherComp :type "PrimitiveComponent Object Reference") (OtherBodyIndex :type Integer))
  (cast `PlayerPawn` OtherActor)
  (goto _label :!via `Reverse`))

(event `self.Sphere.OnComponentHit`
  (params (HitComponent :type "PrimitiveComponent Object Reference") (OtherActor :type "Actor Object Reference") (OtherComp :type "PrimitiveComponent Object Reference") (NormalImpulse :type "Vector Structure") (Hit :type "HitResult Structure (by ref)"))
  (bind _sphere (`self.Sphere`))
  (bind _returnvalue (* (`SceneComponent.GetComponentVelocity` _sphere) (`PrimitiveComponent.GetMass` _sphere)))
  (bind _asplayer_pawn (cast `PlayerPawn` OtherActor))
  (`PlayerPawn.ApplyDamage` _asplayer_pawn (/ (`KismetMathLibrary.VSize` _returnvalue) 7000.0))
  (`/Engine/EditorBlueprintResources/StandardMacros.IsValid` OtherComp
    (:`Is Valid`
      (`PrimitiveComponent.AddImpulse` OtherComp _returnvalue "None" false))
    (:`Is Not Valid`
      _))
  (`PrimitiveComponent.AddImpulse` (`self.Sphere`) (`KismetMathLibrary.ClampVectorSize` (* _returnvalue (`KismetMathLibrary.Conv_DoubleToVector` -4.0)) 250000.0 1000000.0) "None" false))

(event `self.ReceiveDestroyed`
  (`GameplayStatics.PlaySoundAtLocation` "/Game/Audio/Enemies/Splinker/SC_Death.SC_Death" (`SceneComponent.K2_GetComponentLocation` (`self.RootComponent`)) (struct) 1.0 1.0 0.0 null null null null)
  (for _ (range 11)
    (`|SpawnActorFromClass` "/Game/Blueprints/BP_FleshPiece.BP_FleshPiece_C" (`KismetMathLibrary.MakeTransform` (+ (`self.K2_GetActorLocation`) (0.0 0.0 20.0))) "AlwaysSpawn" "OverrideRootScale" null null)))

(fn `UserConstructionScript`)